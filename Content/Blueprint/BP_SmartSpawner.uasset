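; BP_SmartSpawner spawns a BP_Stem_Target at BeginPlay when the VRPawn's current mode is Angle Sniper.
; With a room mesh, it picks a random MRUK wall position and orients the target along the surface normal.
; Otherwise it uses a random point in FallbackBox, with rotation computed toward the player from a separately rolled point.
; Despite the SpawnTargetLoop name, the repeat timer is unconnected, so spawning runs once.
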(event Custom|SpawnTargetLoop
  (bind _returnvalue (Subsystems|GetMRUKSubsystem))
  (bind _fallbackbox (Variables|Default|GetFallbackBox))
  (bind _returnvalue_2 (Class|MRUKSubsystem|GetCurrentRoom _returnvalue))
  (bind _returnvalue_3 (Transformation|GetWorldLocation _fallbackbox))
  (bind _returnvalue_4 (Components|Box|GetScaledBoxExtent _fallbackbox))
  (bind _returnvalue_5 (Math|Random|RandomPointinBoundingBox _returnvalue_3 _returnvalue_4))
  (bind _asvrpawn (Utilities|Casting|CastToVRPawn (Game|Player|GetPlayerPawn 0)))
  (switch Utilities|FlowControl|Switch|SwitchonE_AppModes (Variables|/Game/VRTemplate/Blueprints/VRPawn.VRPawn_C|GetCurrentMode _asvrpawn)
    (:NewEnumerator1
      (if (Variables|Default|GetbHasRoomMesh)
        (Development|PrintString "Room")
        (Utilities|IsValid _returnvalue_2
          (:Is%20Valid
            (bind (_outposition _outnormal _returnvalue_6) (Class|MRUKRoom|GenerateRandomPositiononSurface _returnvalue_2 "AnySurface" 0.0 (Utilities|Struct|MakeMRUKLabelFilter (Utilities|Array|MakeArray "WALL_FACE") 0 7)))
            (if _returnvalue_6
              (Game|SpawnActorfromClass "/Game/Blueprint/BP_Stem_Target.BP_Stem_Target_C" (Math|Transform|MakeTransform _outposition (Math|Conversions|RotationFromXVector _outnormal) "1.000000,1.000000,1.000000") "AdjustIfPossibleButAlwaysSpawn" "MultiplyWithRoot" 0 0)))
          (:Is%20Not%20Valid
            (Development|PrintString "Room NOT fOUND")))
        (else
          (Development|PrintString "fake")
          (Game|SpawnActorfromClass "/Game/Blueprint/BP_Stem_Target.BP_Stem_Target_C" (Math|Transform|MakeTransform _returnvalue_5 (Math|Rotator|FindLookatRotation _returnvalue_5 (Transformation|GetActorLocation (Game|Player|GetPlayerPawn 0))) "1.000000,1.000000,1.000000") "AdjustIfPossibleButAlwaysSpawn" "MultiplyWithRoot" 0 0))))))

(event EventBeginPlay
  (CallFunction|SpawnTargetLoop))

(fn ConstructionScript)