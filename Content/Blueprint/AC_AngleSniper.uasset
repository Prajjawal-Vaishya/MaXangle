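; VR pawn component for an angle-and-power sniper exercise that launches physics balls from the stylus tip toward a stem target.
; Analog trigger input maps to launch power, which sets the spawned ball's velocity along the stylus forward vector.
; Trajectory updates feed speed, pitch and target distance to a holographic HUD, drawing horizontal and vertical velocity debug arrows.
; The predicted-path debug draw uses the unscaled forward vector, ignoring launch power.
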(event Custom|UpdateAnalogPower
  (params (RawTriggerValue :type Float%20%28double-precision%29))
  (Variables|Default|SetLaunchPower (Math|Float|MapRangeClamped RawTriggerValue 0.0 1.0 5e+02 2.5e+03)))

(event Custom|UpdateTrajectory
  (bind _activestylus (Variables|Default|GetActiveStylus))
  (bind _activestylus_2 (Variables|Default|GetActiveStylus))
  (bind _activestylus_3 (Variables|Default|GetActiveStylus))
  (bind _returnvalue (Math|Vector|GetForwardVector _activestylus_3))
  (bind _returnvalue_2 (Transformation|GetWorldLocation _activestylus_3))
  (bind _asbp_angle_sniper_hud (Utilities|Casting|CastToBP_AngleSniperHUD (UserInterface|GetUserWidgetObject (Variables|Default|GetHolo%20HUD))))
  (Default|UpdateSniperData _asbp_angle_sniper_hud (/ (Variables|Default|GetLaunchPower) 1e+02) (.pitch (Transformation|GetWorldRotation _activestylus_2)) (/ (Math|Vector|Distance(Vector) (Transformation|GetWorldLocation _activestylus_2) (Transformation|GetActorLocation (Variables|Default|GetTargetRef))) 1e+02))
  (Class|GameplayStatics|BlueprintPredictProjectilePathbyTraceChannel (Transformation|GetWorldLocation _activestylus) (Math|Vector|GetForwardVector _activestylus) true 0.0 "ECC_Visibility" false 0 "ForOneFrame")
  (Utilities|FlowControl|Sequence
    (:then_0
      (Rendering|Debug|DrawDebugArrow _returnvalue_2 (+ _returnvalue_2 (* (Math|Vector|MakeVector (.x _returnvalue) (.y _returnvalue) 0.0) (Variables|Default|GetLaunchPower))) 4e+01 "(R=0.798958,G=0.000000,B=0.116371,A=1.000000)" 0.05 3.0))
    (:then_1
      (Rendering|Debug|DrawDebugArrow _returnvalue_2 (+ _returnvalue_2 (* (Math|Vector|MakeVector 0.0 0.0 (.z _returnvalue)) (Variables|Default|GetLaunchPower))) 4e+01 "(R=0.020819,G=0.000000,B=1.000000,A=1.000000)" 0.05 3.0))))

(event Custom|FireProjectile
  (bind _activestylus (Variables|Default|GetActiveStylus))
  (bind _returnvalue (Game|SpawnActorfromClass "/Game/Blueprint/BP_PhysicsBall.BP_PhysicsBall_C" (Transformation|GetWorldTransform _activestylus) "Undefined" "MultiplyWithRoot" 0 0))
  (Physics|SetPhysicsLinearVelocity (Variables|/Game/Blueprint/BP_PhysicsBall.BP_PhysicsBall_C|GetBall _returnvalue) (* (Math|Vector|GetForwardVector _activestylus) (Variables|Default|GetLaunchPower)) false "None"))

(event EventBeginPlay
  (bind _asvrpawn (Utilities|Casting|CastToVRPawn (Components|GetOwner)))
  (Variables|Default|SetActiveStylus (Variables|/Game/VRTemplate/Blueprints/VRPawn.VRPawn_C|GetStylusTip _asvrpawn))
  (Variables|Default|SetHolo%20HUD (Variables|/Game/VRTemplate/Blueprints/VRPawn.VRPawn_C|GetHoloHUD _asvrpawn))
  (bind _returnvalue (Actor|GetActorOfClass "/Game/Blueprint/BP_Stem_Target.BP_Stem_Target_C"))
  (Variables|Default|SetTargetRef _returnvalue))