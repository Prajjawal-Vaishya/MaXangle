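; Actor component that builds geometric shapes point by point from trigger presses, drawing each edge as a stretched static mesh between points.
; A three-state machine places the first point and edge, then accepts further points only at a valid corner angle, closing the shape after enough sides.
; Tick validates that angle against a target with tolerance using a dot product.
; Tip smoothing and snapping are not computed here, and shape cycling is an empty stub.
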(event Custom|TriggeredPressed
  (bind _placedpoints (Variables|Default|GetPlacedPoints))
  (bind _placedpoints_2 (Variables|Default|GetPlacedPoints))
  (bind _smoothedtiplocation (Variables|Default|GetSmoothedTipLocation))
  (bind _placedpoints_3 (Variables|Default|GetPlacedPoints))
  (switch int (Variables|Default|GetBuilderState)
    (:0
      (Utilities|Array|Add _placedpoints _smoothedtiplocation)
      (Variables|Default|SetBuilderState 1))
    (:1
      (Utilities|Array|Add _placedpoints _smoothedtiplocation)
      (bind _point (CallFunction|GetLastPoint _placedpoints_3))
      (bind _point_2 (CallFunction|GetPreviousPoint _placedpoints_3))
      (CallFunction|SpawnEdge _point_2 _point)
      (Variables|Default|SetBuilderState 2))
    (:2
      (if (Variables|Default|GetbIsAngleValid)
        (Utilities|Array|Add _placedpoints_3 (Variables|Default|GetSnappedLocation))
        (bind _point_3 (CallFunction|GetLastPoint _placedpoints_3))
        (bind _point_4 (CallFunction|GetPreviousPoint _placedpoints_3))
        (CallFunction|SpawnEdge _point_4 _point_3)
        (bind _output_get (Variables|Default|SetEdgeCount (+ (Variables|Default|GetEdgeCount) 1)))
        (if (>= _output_get (Variables|Default|GetNumberOfSides))
          (bind _point_5 (CallFunction|GetLastPoint _placedpoints_2))
          (CallFunction|SpawnEdge _point_5 (Utilities|Array|Get(acopy) _placedpoints_2))
          (Development|PrintString "Shape Complete! [CurrentShape]")
          (Variables|Default|SetBuilderState 0)
          (Variables|Default|SetEdgeCount 0)
          (Utilities|Array|Clear (Variables|Default|GetPlacedPoints))
          (Utilities|Array|Clear (Variables|Default|GetPlacedEdges)))))))

(event Custom|CycleShape)

(event EventTick
  (params (DeltaSeconds :type Float%20%28single-precision%29))
  (bind _placedpoints (Variables|Default|GetPlacedPoints))
  (bind _targetangle (Variables|Default|GetTargetAngle))
  (bind _angletolerance (Variables|Default|GetAngleTolerance))
  (bind _point (CallFunction|GetLastPoint _placedpoints))
  (bind _point_2 (CallFunction|GetPreviousPoint _placedpoints))
  (if (== (Variables|Default|GetBuilderState) 2)
    (bind _output_get (Variables|Default|SetSmoothedAngle (Class|KismetMathLibrary|DegAcos (Math|Vector|DotProduct (Math|Vector|Normalize (- _point_2 _point)) (Math|Vector|Normalize (- (Variables|Default|GetSmoothedTipLocation) ""))))))
    (if (Math|Float|InRange(Float) _output_get (- _targetangle _angletolerance) (+ _targetangle _angletolerance))
      (Development|PrintString "ANGLE VALIDATED: 90°" true true "(R=0.000000,G=1.000000,B=0.169848,A=1.000000)" 1.0 "AngleHUD")
      (Variables|Default|SetbIsAngleValid true)
      (else
        (Development|PrintString (Utilities|String|ToString(Float) _output_get) true true "(R=1.000000,G=0.000000,B=0.184105,A=1.000000)")
        (Variables|Default|SetbIsAngleValid false)))))

(fn ConstructionScript)

(fn SpawnEdge
  (params (StartPoint :type Vector) (EndPoint :type Vector))
  (bind _output_get (LocalVariables|SetMidpoint (/ (+ StartPoint EndPoint) 2.0)))
  (bind _returnvalue (AddComponent|AddStaticMeshComponent false))
  (Transformation|SetWorldLocationAndRotation _returnvalue _output_get (Math|Rotator|FindLookatRotation StartPoint EndPoint) false false)
  (Transformation|SetWorldScale3D _returnvalue (Math|Vector|MakeVector (/ (Math|Vector|Distance(Vector) StartPoint EndPoint) 1e+02) 0.02 0.02))
  (Utilities|Array|Add (Variables|Default|GetPlacedEdges) _returnvalue))

(fn GetPreviousPoint
  (params (Array :type Array%20of%20Vectors))
  (return (Utilities|Array|Get(acopy) Array (- (Utilities|Array|LastIndex Array) 1))))

(fn GetLastPoint
  (params (Array :type Array%20of%20Vectors))
  (return (Utilities|Array|Get(acopy) Array (Utilities|Array|LastIndex Array))))

(fn GetTrueTipLocation)