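; VR pawn component that lets the player build polygons point by point, validating each new corner against the selected shape's target angle.
; A three-state press handler places lettered joints and stretched-cube edges, then auto-closes the shape once the edge count reaches the side count.
; Tick feeds live length, angle and validity to the pawn's hologram protractor.
; World-space labels, rotated toward the camera on spawn, show lengths and corner angles.
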(event Custom|TriggeredPressed
  (params (GeometrySelect :type Integer))
  (bind _placedpoints (Variables|Default|GetPlacedPoints))
  (bind _placedpoints_2 (Variables|Default|GetPlacedPoints))
  (bind _smoothedtiplocation (Variables|Default|GetSmoothedTipLocation))
  (bind _placedpoints_3 (Variables|Default|GetPlacedPoints))
  (bind _point (CallFunction|GetPreviousPoint _placedpoints_2))
  (bind _point_2 (CallFunction|GetLastPoint _placedpoints_3))
  (bind _point_3 (CallFunction|GetPreviousPoint _placedpoints_3))
  (bind _point_4 (CallFunction|GetLastPoint _placedpoints_2))
  (bind _output (Utilities|Array|Get(acopy) _placedpoints_2))
  (bind _output_2 (Utilities|Array|Get(acopy) _placedpoints_2 1))
  (Variables|Default|SetNumberOfSides (Utilities|Array|Get(acopy) (Variables|Default|GetAllNumberOfSides) GeometrySelect))
  (Variables|Default|SetTargetAngle (Utilities|Array|Get(acopy) (Variables|Default|GetAllAngle) GeometrySelect))
  (switch int (Variables|Default|GetBuilderState)
    (:0
      (bind _returnvalue (Utilities|Array|Add _placedpoints _smoothedtiplocation))
      (CallFunction|SpawnVector (Utilities|Array|Get(acopy) _placedpoints _returnvalue))
      (Variables|Default|SetBuilderState 1))
    (:1
      (bind _returnvalue_2 (Utilities|Array|Add _placedpoints _smoothedtiplocation))
      (CallFunction|SpawnVector (Utilities|Array|Get(acopy) _placedpoints _returnvalue_2))
      (CallFunction|SpawnEdge (CallFunction|GetPreviousPoint _placedpoints_3) (CallFunction|GetLastPoint _placedpoints_3))
      (Variables|Default|SetBuilderState 2))
    (:2
      (if (Variables|Default|GetbIsAngleValid)
        (bind _returnvalue_3 (Utilities|Array|Add _placedpoints_3 (Variables|Default|GetSmoothedTipLocation)))
        (CallFunction|SpawnVector (Utilities|Array|Get(acopy) _placedpoints_3 _returnvalue_3))
        (CallFunction|SpawnEdge _point_3 _point_2)
        (CallFunction|SpawnAngleHologram (CallFunction|GetAnglePoint) _point_3 _point_2 (stale EventTick _output_get))
        (bind _output_get (Variables|Default|SetEdgeCount (+ (Variables|Default|GetEdgeCount) 1)))
        (if (>= _output_get (Variables|Default|GetNumberOfSides))
          (CallFunction|SpawnEdge _point_4 _output)
          (CallFunction|SpawnAngleHologram _point _point_4 _output (.OutAngle (Class|MaXangleMathLibrary|GetGeometryData _point _point_4 _output 0.0 0.0)))
          (CallFunction|SpawnAngleHologram _point_4 _output _output_2 (.OutAngle (Class|MaXangleMathLibrary|GetGeometryData _point_4 _output _output_2 0.0 0.0)))
          (Variables|Default|SetBuilderState 0)
          (Variables|Default|SetEdgeCount 0)
          (Utilities|Array|Clear (Variables|Default|GetPlacedPoints))
          (Utilities|Array|Clear (Variables|Components|GetPlacedEdges)))))))

(event EventTick
  (params (DeltaSeconds :type Float%20%28single-precision%29))
  (bind _placedpoints (Variables|Default|GetPlacedPoints))
  (bind _smoothedtiplocation (Variables|Default|GetSmoothedTipLocation))
  (bind _targetangle (Variables|Default|GetTargetAngle))
  (bind _angletolerance (Variables|Default|GetAngleTolerance))
  (bind _point (CallFunction|GetLastPoint _placedpoints))
  (bind _point_2 (CallFunction|GetPreviousPoint _placedpoints))
  (bind (_outangle _outedgelength_cm _boutisvalid) (Class|MaXangleMathLibrary|GetGeometryData _point_2 _point _smoothedtiplocation _targetangle _angletolerance))
  (if (== (Variables|Default|GetBuilderState) 2)
    (bind _output_get (Variables|Default|SetSmoothedAngle _outangle))
    (Variables|Default|SetbIsAngleValid _boutisvalid)
    (bind _asvrpawn (Utilities|Casting|CastToVRPawn (Components|GetOwner)))
    (bind _aswbp_hologram_protractor (Utilities|Casting|CastToWBP_HologramProtractor (UserInterface|GetUserWidgetObject (Variables|/Game/VRTemplate/Blueprints/VRPawn.VRPawn_C|GetProtractorHologram _asvrpawn))))
    (Default|UpdateDisplay _aswbp_hologram_protractor (Variables|Default|GetSmoothedAngle) (Variables|Default|GetTargetAngle) _outedgelength_cm _boutisvalid)
    (elif (== (Variables|Default|GetBuilderState) 1)
      (bind _asvrpawn_2 (Utilities|Casting|CastToVRPawn (Components|GetOwner)))
      (bind _aswbp_hologram_protractor_2 (Utilities|Casting|CastToWBP_HologramProtractor (UserInterface|GetUserWidgetObject (Variables|/Game/VRTemplate/Blueprints/VRPawn.VRPawn_C|GetProtractorHologram _asvrpawn_2))))
      (Default|UpdateDisplay _aswbp_hologram_protractor_2 0.0 0.0 (/ (Math|Vector|Distance(Vector) (CallFunction|GetLastPoint (Variables|Default|GetPlacedPoints)) (Variables|Default|GetSmoothedTipLocation)) 1e+02) false))))

(fn SpawnEdge
  (params (StartPoint :type Vector) (EndPoint :type Vector))
  (bind _returnvalue (Math|Vector|Distance(Vector) StartPoint EndPoint))
  (bind _returnvalue_2 (Components|GetOwner))
  (bind _returnvalue_3 (/ _returnvalue 1e+02))
  (bind _output_get (LocalVariables|SetMidpoint (/ (+ StartPoint EndPoint) 2.0)))
  (bind _returnvalue_4 (Game|AddComponentbyClass _returnvalue_2 "/Script/Engine.StaticMeshComponent" false))
  (Components|StaticMesh|SetStaticMesh _returnvalue_4 "/Game/StarterContent/Shapes/Shape_Cube.Shape_Cube")
  (Rendering|Material|SetMaterial _returnvalue_4 0 "/Game/Material/M_Hologram_STEM.M_Hologram_STEM")
  (Transformation|SetWorldLocationAndRotation _returnvalue_4 _output_get (Math|Rotator|FindLookatRotation StartPoint EndPoint) false false)
  (Transformation|SetWorldScale3D _returnvalue_4 (Math|Vector|MakeVector _returnvalue_3 0.02 0.02))
  (Utilities|Array|Add (Variables|Components|GetPlacedEdges) 0)
  (bind _returnvalue_5 (Game|AddComponentbyClass _returnvalue_2 "/Script/UMG.WidgetComponent" false))
  (Transformation|SetWorldScale3D _returnvalue_5 "0.100000,0.100000,0.100000")
  (Transformation|SetWorldRotation _returnvalue_5 (Math|Rotator|FindLookatRotation _output_get (Camera|GetCameraLocation (Game|GetPlayerCameraManager 0))) false false)
  (bind _returnvalue_6 (UserInterface|CreateWidget "/Game/UI/W_FloatingLabel.W_FloatingLabel_C"))
  (UserInterface|SetWidget _returnvalue_5 _returnvalue_6)
  (Variables|/Game/UI/W_FloatingLabel.W_FloatingLabel_C|SetLabelText _returnvalue_6 (Utilities|String|ToString(Text) (Utilities|Text|FormatText "{Len} m" (Utilities|Text|ToText(Float) _returnvalue_3 "HalfToEven"))))
  (Transformation|SetWorldLocation _returnvalue_5 (+ _output_get (Math|Vector|MakeVector 0.0 0.0 0.0)) false false)
  (Class|WidgetComponent|SetWidgetSpace _returnvalue_5 "World")
  (Class|WidgetComponent|SetDrawatDesiredSize _returnvalue_5 true))

(fn GetPreviousPoint
  (params (Array :type Array%20of%20Vectors))
  (return (Utilities|Array|Get(acopy) Array (- (Utilities|Array|LastIndex Array) 1))))

(fn GetLastPoint
  (params (Array :type Array%20of%20Vectors))
  (return (Utilities|Array|Get(acopy) Array (Utilities|Array|LastIndex Array))))

(fn SpawnVector
  (params (VectorLocation :type Vector))
  (bind _returnvalue (Components|GetOwner))
  (bind _returnvalue_2 (Game|AddComponentbyClass _returnvalue "/Script/Engine.StaticMeshComponent" false))
  (Components|StaticMesh|SetStaticMesh _returnvalue_2 "/Game/StarterContent/Shapes/Shape_Sphere.Shape_Sphere")
  (Rendering|Material|SetMaterial _returnvalue_2 0 "/Game/Material/M_Solid_Joint.M_Solid_Joint")
  (Transformation|SetWorldLocationAndRotation _returnvalue_2 VectorLocation "0, 0, 0" false false)
  (Transformation|SetWorldScale3D _returnvalue_2 (Math|Vector|MakeVector 0.06 0.06 0.06))
  (bind _returnvalue_3 (Utilities|Array|Add (Variables|Components|GetPlaceVector) _returnvalue_2))
  (bind _returnvalue_4 (Game|AddComponentbyClass _returnvalue "/Script/UMG.WidgetComponent" false))
  (Transformation|SetWorldScale3D _returnvalue_4 "0.200000,0.200000,0.200000")
  (Transformation|SetWorldRotation _returnvalue_4 (Math|Rotator|FindLookatRotation VectorLocation (Camera|GetCameraLocation (Game|GetPlayerCameraManager 0))) false false)
  (bind _returnvalue_5 (UserInterface|CreateWidget "/Game/UI/W_FloatingLabel.W_FloatingLabel_C"))
  (UserInterface|SetWidget _returnvalue_4 _returnvalue_5)
  (Variables|/Game/UI/W_FloatingLabel.W_FloatingLabel_C|SetLabelText _returnvalue_5 (Utilities|Array|Get(acopy) (Variables|Default|GetAlphabet) _returnvalue_3))
  (Transformation|SetWorldLocation _returnvalue_4 VectorLocation false false)
  (Class|WidgetComponent|SetWidgetSpace _returnvalue_4 "World")
  (Class|WidgetComponent|SetDrawatDesiredSize _returnvalue_4 true))

(fn GetAngleTextLocation
  (params (Point%201 :type Vector) (Corner%20Point :type Vector) (Point%202 :type Vector) (Inside%20Depth :type Float%20%28double-precision%29))
  (return (+ (+ Corner%20Point (* (Math|Vector|Normalize (+ (Math|Vector|Normalize (- Point%201 Corner%20Point)) (Math|Vector|Normalize (- Point%202 Corner%20Point)))) Inside%20Depth)) (Math|Vector|MakeVector 0.0 0.0 0.0))))

(fn SpawnAngleHologram
  (params (Point%20A :type Vector) (Corner%20B :type Vector) (Point%20C :type Vector) (LockedAngle :type Float%20%28double-precision%29))
  (bind _text_location (CallFunction|GetAngleTextLocation Point%20A Corner%20B Point%20C 1e+01))
  (bind _returnvalue (Game|AddComponentbyClass (Components|GetOwner) "/Script/UMG.WidgetComponent" false))
  (Transformation|SetWorldScale3D _returnvalue "0.100000,0.100000,0.100000")
  (Transformation|SetWorldRotation _returnvalue (Math|Rotator|FindLookatRotation _text_location (Camera|GetCameraLocation (Game|GetPlayerCameraManager 0))) false false)
  (bind _returnvalue_2 (UserInterface|CreateWidget "/Game/UI/W_FloatingLabel.W_FloatingLabel_C"))
  (UserInterface|SetWidget _returnvalue _returnvalue_2)
  (Variables|/Game/UI/W_FloatingLabel.W_FloatingLabel_C|SetLabelText _returnvalue_2 (Utilities|String|ToString(Text) (Utilities|Text|FormatText "{Ang}°" (Utilities|Text|ToText(Float) LockedAngle "HalfToEven" false false 1 324 1 1))))
  (Transformation|SetWorldLocation _returnvalue _text_location false false)
  (Class|WidgetComponent|SetWidgetSpace _returnvalue "World")
  (Class|WidgetComponent|SetDrawatDesiredSize _returnvalue true))

(fn GetAnglePoint
  (bind _placedpoints (Variables|Default|GetPlacedPoints))
  (return (Utilities|Array|Get(acopy) _placedpoints (- (Utilities|Array|LastIndex _placedpoints) 2))))

(fn AngleCal
  (params (PointStart :type Vector) (PointMid :type Vector) (PointEnd :type Vector))
  (return (Class|KismetMathLibrary|DegAcos (Math|Vector|DotProduct (Math|Vector|Normalize (- PointStart PointMid)) (Math|Vector|Normalize (- PointEnd PointMid))))))